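; Spawner actor that periodically spawns a random actor class from an ActorsToSpawn list, set per instance in the level.
; BeginPlay starts a looping timer at SpawnFrequency that calls Spawn.
; Spawn picks one of ten spawn-point components at random for the location, then spawns a random entry from the list there.
; The debug print re-rolls its random index, so it may not match the spawned entry.
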(event Custom|Spawn
  (bind _actorstospawn (Variables|Settings|GetActorsToSpawn))
  (bind _returnvalue (Utilities|Array|Length _actorstospawn))
  (bind _returnvalue_2 (- _returnvalue 1))
  (bind _returnvalue_3 (Math|Random|RandomIntegerinRange 0 _returnvalue_2))
  ;[1 1 1] Initiates Spawn Sequence
  (Utilities|FlowControl|Sequence
    (:then_0
      ;[1 1 1] Getting and setting random spawn location.
      (switch int (Math|Random|RandomIntegerinRange 1 10)
        (:1
          (Variables|Default|SetSpawnLocation (Transformation|GetWorldLocation (Variables|Default|GetSP1))))
        (:2
          (Variables|Default|SetSpawnLocation (Transformation|GetWorldLocation (Variables|Default|GetSP2))))
        (:3
          (Variables|Default|SetSpawnLocation (Transformation|GetWorldLocation (Variables|Default|GetSP3))))
        (:4
          (Variables|Default|SetSpawnLocation (Transformation|GetWorldLocation (Variables|Default|GetSP4))))
        (:5
          (Variables|Default|SetSpawnLocation (Transformation|GetWorldLocation (Variables|Default|GetSP5))))
        (:6
          (Variables|Default|SetSpawnLocation (Transformation|GetWorldLocation (Variables|Default|GetSP6))))
        (:7
          (Variables|Default|SetSpawnLocation (Transformation|GetWorldLocation (Variables|Default|GetSP7))))
        (:8
          (Variables|Default|SetSpawnLocation (Transformation|GetWorldLocation (Variables|Default|GetSP8))))
        (:9
          (Variables|Default|SetSpawnLocation (Transformation|GetWorldLocation (Variables|Default|GetSP9))))
        (:10
          (Variables|Default|SetSpawnLocation (Transformation|GetWorldLocation (Variables|Default|GetSP10))))))
    (:then_1
      ;[1 1 1] Spawns actor from list of available actors. This is set by selecting the spawner in the level and adding actors.
      (Game|SpawnActorfromClass (Utilities|Array|Get(acopy) _actorstospawn _returnvalue_3) (Math|Transform|MakeTransform (Variables|Default|GetSpawnLocation) "0, 0, 0" "1,1,1") "Undefined" 0 0)
      (Development|PrintString (Utilities|String|ToString(Integer) _returnvalue_3)))))

(event EventBeginPlay
  (Utilities|Time|SetTimerbyFunctionName 0 "Spawn" (Variables|Settings|GetSpawnFrequency) true))

(fn ConstructionScript)