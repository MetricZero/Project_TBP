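; Succubus player character Blueprint that keeps the pawn moving automatically on the horizontal plane, relative to the camera's control yaw.
; W and D press and release set GoingUp and GoingRight flags.
; While a flag is set, the MoveForward or MoveRight axis event pushes forward or right.
; Otherwise, Tick pushes backward or left, so movement input never rests on either axis.
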(event EventBeginPlay)

(event Collision|EventActorBeginOverlap
  (params (OtherActor :type Actor%20Object%20Reference)))

(fn ConstructionScript)

(event EventTick
  (params (DeltaSeconds :type Float%20%28single-precision%29))
  (bind _returnvalue (Pawn|GetControlRotation :!class /Script/Engine.Pawn))
  (bind _yaw (Math|Rotator|BreakRotator _returnvalue))
  (bind _returnvalue_2 (Math|Rotator|MakeRotator 0.0 0.0 _yaw))
  ;[1 1 1] Automatic Movement (There's a simpler way to do this but this works so meh)
  (Utilities|FlowControl|Sequence
    (:then_0
      (if (not (Variables|Default|GetGoingUp?))
        (Pawn|Input|AddMovementInput (Math|Vector|GetForwardVector _returnvalue_2) -1.0 false)))
    (:then_1
      (if (not (Variables|Default|GetGoingRight?))
        (Pawn|Input|AddMovementInput (Math|Vector|GetRightVector _returnvalue_2) -1.0 false)))))

(event Input|AxisEvents|InputAxisMoveForward
  (params (AxisValue :type Float%20%28single-precision%29))
  ;[1 1 1] Up Movement
  (if (Variables|Default|GetGoingUp?)
    (Pawn|Input|AddMovementInput (Math|Vector|GetForwardVector (Math|Rotator|MakeRotator 0.0 0.0 (.Yaw (Math|Rotator|BreakRotator (Pawn|GetControlRotation :!class /Script/Engine.Pawn))))) 1.0 false)))

(event Input|AxisEvents|InputAxisMoveRight
  (params (AxisValue :type Float%20%28single-precision%29))
  ;[1 1 1] Down Movement
  (if (Variables|Default|GetGoingRight?)
    (Pawn|Input|AddMovementInput (Math|Vector|GetRightVector (Math|Rotator|MakeRotator 0.0 0.0 (.Yaw (Math|Rotator|BreakRotator (Pawn|GetControlRotation :!class /Script/Engine.Pawn))))) 1.0 false)))

(event Input|KeyboardEvents|W
  (params (Key :type Key%20Structure))
  ;[1 1 1] Up Movement
  (:Pressed
    (Variables|Default|SetGoingUp? true))
  (:Released
    (Variables|Default|SetGoingUp? false)))

(event Input|KeyboardEvents|D
  (params (Key :type Key%20Structure))
  ;[1 1 1] Down Movement
  (:Pressed
    (Variables|Default|SetGoingRight? true))
  (:Released
    (Variables|Default|SetGoingRight? false)))